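; Game mode Blueprint that tallies the level's collectables when play begins.
; BeginPlay counts all Collectables_BP actors, stores the result as both remaining and total, and prints the total.
; Two disconnected chains never run: a one-second countdown step that shows DeathScreen and disables Parkour_char_bp input at zero, and a delayed DefaultWidget display.
; Tick and the construction script are empty.
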(event `self.ReceiveBeginPlay`
  (bind _outactors (`GameplayStatics.GetAllActorsOfClass` "/Game/Blueprints/Collectables_BP.Collectables_BP_C"))
  (bind _output_get (set `self.CollectablesLeft` (`KismetArrayLibrary.Array_Length` _outactors)))
  (bind _output_get_2 (set `self.TotalCollectables` _output_get))
  (`KismetSystemLibrary.PrintString` (`KismetStringLibrary.Conv_IntToString` _output_get_2)))

(fn `UserConstructionScript`)