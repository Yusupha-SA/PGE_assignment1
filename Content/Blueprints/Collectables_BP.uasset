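; Collectable pickup actor that the parkour character collects by pressing R while inside its box.
; Box overlap with Parkour_char_bp toggles the actor's input on and off.
; Pressing R decrements CollectablesLeft on the GameMode, adds a Collectable_WB widget to the viewport and destroys the actor.
; BeginPlay prints the GameInstance_p Collectables count; an unconnected branch that resets it and opens Level1 never runs.
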(event `Key|R`
  (params (Key :type "Key Structure"))
  (:`Pressed`
    (bind _asgame_mode (cast `/Game/Blueprints/GameMode` (`GameplayStatics.GetGameMode`)))
    (bind _result (`/Engine/EditorBlueprintResources/StandardMacros.DecrementInt` (`/Game/Blueprints/GameMode.CollectablesLeft` _asgame_mode))
      (:`  `
        (set `/Game/Blueprints/GameMode.CollectablesLeft` _result _asgame_mode)
        (bind _returnvalue (`|CreateWidget` "/Game/UI/Collectable_WB.Collectable_WB_C"))
        (`UserWidget.AddToViewport` _returnvalue 0)
        (`self.K2_DestroyActor`)))))

(event `self.ReceiveBeginPlay`
  (bind _asgame_instance_p (cast `/Game/Blueprints/GameInstance_p` (`GameplayStatics.GetGameInstance`)))
  (`KismetSystemLibrary.PrintString` (`KismetStringLibrary.Conv_IntToString` (`/Game/Blueprints/GameInstance_p.Collectables` _asgame_instance_p))))

(event `self.Box.OnComponentBeginOverlap`
  (params (OverlappedComponent :type "PrimitiveComponent Object Reference") (OtherActor :type "Actor Object Reference") (OtherComp :type "PrimitiveComponent Object Reference") (OtherBodyIndex :type Integer) (bFromSweep :type Boolean) (SweepResult :type "HitResult Structure (by ref)"))
  (cast `/Game/Blueprints/Parkour_char_bp` OtherActor)
  (`self.EnableInput` (`GameplayStatics.GetPlayerController` 0)))

(event `self.Box.OnComponentEndOverlap`
  (params (OverlappedComponent :type "PrimitiveComponent Object Reference") (OtherActor :type "Actor Object Reference") (OtherComp :type "PrimitiveComponent Object Reference") (OtherBodyIndex :type Integer))
  (cast `/Game/Blueprints/Parkour_char_bp` OtherActor)
  (`self.DisableInput` (`GameplayStatics.GetPlayerController` 0)))

(fn `UserConstructionScript`)